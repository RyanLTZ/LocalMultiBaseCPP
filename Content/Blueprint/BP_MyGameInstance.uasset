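; Game instance Blueprint that hosts and joins LAN multiplayer sessions.
; Hosting creates a four-slot LAN session and, on success, opens the Main map as a listen server.
; Joining searches for LAN sessions and calls JoinSession on every result while storing it.
; After the loop, it passes the stored result to LMPlayerController's JoinWithSearchResult.
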(event `HostAdvancedSession`
  (`CreateSessionCallbackProxy.CreateSession` (`GameplayStatics.GetPlayerController` 0) 4 true
    (:`OnSuccess`
      (`GameplayStatics.OpenLevel` "Main?listen"))))

(event `FindAndJoinLANGame`
  (bind _returnvalue (`GameplayStatics.GetPlayerController` 0))
  (bind _results (`FindSessionsCallbackProxy.FindSessions` (`GameplayStatics.GetPlayerController` 0) 32 true)
    (:`OnSuccess`
      (for _array_element _results
        (set `self.Array Element` _array_element)
        (`JoinSessionCallbackProxy.JoinSession` _returnvalue _array_element))
      (bind _aslmplayer_controller (cast `LMPlayerController` _returnvalue))
      (`LMPlayerController.BP_JoinWithSearchResult` _aslmplayer_controller (`self.Array Element`)))))