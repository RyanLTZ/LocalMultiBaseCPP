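; BP_Bullet is a projectile that flies straight along its forward vector and can destroy destructable obstacles.
; Tick moves it by a speed variable scaled by delta time, without sweeping, so hits come from actor overlap events.
; Overlapping a BP_Obstacle destroys only the bullet, while a BP_DestructableObs is destroyed along with it.
; Overlaps with any other actor are ignored.
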(event `self.ReceiveTick`
  (params (DeltaSeconds :type "Float (single-precision)"))
  (`self.K2_SetActorLocation` (+ (`self.K2_GetActorLocation`) (* (* (`self.GetActorForwardVector`) (`self.MoveSpeed_0`)) DeltaSeconds))))

(event `self.ReceiveActorBeginOverlap`
  (params (OtherActor :type "Actor Object Reference"))
  (cast `/Game/Blueprints/BP_Obstacle` OtherActor
    (:`then`
      _)
    (:`CastFailed`
      (bind _asbp_destructable_obs (cast `/Game/Blueprints/BP_DestructableObs` OtherActor))
      (`self.K2_DestroyActor` _asbp_destructable_obs)))
  (`self.K2_DestroyActor`))

(fn `UserConstructionScript`)