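; BP_ProceduralTile is an actor that builds a grid of box tiles as one procedural mesh in its construction script.
; It derives tile counts from grid and tile sizes, then offsets each generated box's vertices and triangle indices into shared buffers.
; Both loops use the depth count, so the grid has equal tile counts on each axis.
; The buffers become a single mesh section and are then cleared.
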(fn `UserConstructionScript`
  (`|ExecutionSequence`
    (:`then_0`
      (bind _output_get (set `self.TileCountHorizontal` (`KismetMathLibrary.FTrunc` (/ (`self.GridWidth`) (`self.TileWidth`)))))
      (bind _output_get_2 (set `self.TileCountDepth` (`KismetMathLibrary.FTrunc` (/ (`self.GridLength`) (`self.TileLength`)))))
      (set `self.TileTotalCount` (* _output_get _output_get_2)))
    (:`then_1`
      (for _index (range (`self.TileCountDepth`))
        (for _index_2 (range (`self.TileCountDepth`))
          (bind (_vertices _triangles _normals _uvs _tangents) (`KismetProceduralMeshLibrary.GenerateBoxMesh` (`KismetMathLibrary.MakeVector` (* (`self.TileWidth`) 0.5) (* (`self.TileLength`) 0.5) (* (`self.TileHeight`) 0.5))))
          (for _array_element _triangles
            (`KismetArrayLibrary.Array_Add` (`self.Triangles`) (+ _array_element (`KismetArrayLibrary.Array_Length` (`self.Vertices`)))))
          (for _array_element_2 _vertices
            (`KismetArrayLibrary.Array_Add` (`self.Vertices`) (+ _array_element_2 (`KismetMathLibrary.MakeVector` (* _index_2 (`self.TileWidth`)) (* _index (`self.TileLength`))))))
          (`KismetArrayLibrary.Array_Append` (`self.Normals`) _normals)
          (`KismetArrayLibrary.Array_Append` (`self.UVs`) _uvs)
          (`KismetArrayLibrary.Array_Append` (`self.Tangents`) _tangents))))
    (:`then_2`
      (`ProceduralMeshComponent.CreateMeshSection_LinearColor` :`self` (`self.ProceduralMesh`) :`Vertices` (`self.Vertices`) :`Triangles` (`self.Triangles`) :`Normals` (`self.Normals`) :`UV0` (`self.UVs`) :`Tangents` (`self.Tangents`))
      (`KismetArrayLibrary.Array_Clear` (`self.Vertices`))
      (`KismetArrayLibrary.Array_Clear` (`self.Triangles`))
      (`KismetArrayLibrary.Array_Clear` (`self.Normals`))
      (`KismetArrayLibrary.Array_Clear` (`self.UVs`))
      (`KismetArrayLibrary.Array_Clear` (`self.Tangents`)))))