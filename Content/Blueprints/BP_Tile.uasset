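; BP_Tile is a floor tile that players claim by passing over it, recoloring it per player index and updating that player's score.
; Construction creates a dynamic material instance from M_Base_Inst.
; Overlap start tints that instance for players 0 and 1, but only stores an overlap material for players 2 and 3.
; Overlap end applies the player's material to the mesh and calls UpatePlayerScore.
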(event `self.ReceiveActorBeginOverlap`
  (params (OtherActor :type "Actor Object Reference"))
  (bind _dynamicmaterial (`self.DynamicMaterial`))
  (bind _asbp_lmpawn_player (cast `/Game/Blueprints/BP_LMPawnPlayer` OtherActor))
  (switch `int` (`LMPawnPlayer.GetPlayerIndex` _asbp_lmpawn_player)
    (:`0`
      (`MaterialInstanceDynamic.SetVectorParameterValue` _dynamicmaterial "BaseColor" (struct :`R` 0.322917 :`B` 0.014332 :`A` 1.0)))
    (:`1`
      (`MaterialInstanceDynamic.SetVectorParameterValue` _dynamicmaterial "BaseColor" (struct :`R` 0.029743 :`G` 0.166667 :`B` 0.023788 :`A` 1.0)))
    (:`2`
      (set `self.Material` "/Game/TopDown/Blueprints/OverlapMaterial_3p.OverlapMaterial_3p"))
    (:`3`
      (set `self.Material` "/Game/TopDown/Blueprints/OverlapMaterial_4p.OverlapMaterial_4p"))))

(event `self.ReceiveActorEndOverlap`
  (params (OtherActor :type "Actor Object Reference"))
  (bind _asbp_lmpawn_player (cast `/Game/Blueprints/BP_LMPawnPlayer` OtherActor))
  (bind _returnvalue (`LMPawnPlayer.GetPlayerIndex` _asbp_lmpawn_player))
  (switch `int` _returnvalue
    (:`0`
      (set `self.Material` "/Game/TopDown/Blueprints/Material_1p.Material_1p"))
    (:`1`
      (set `self.Material` "/Game/TopDown/Blueprints/Material_2p.Material_2p"))
    (:`2`
      (set `self.Material` "/Game/TopDown/Blueprints/Material_3p.Material_3p"))
    (:`3`
      (set `self.Material` "/Game/TopDown/Blueprints/Material_4p.Material_4p")))
  (`PrimitiveComponent.SetMaterial` (`self.MeshComponent`) 0 (`self.Material`))
  (`self.UpatePlayerScore` _returnvalue))

(fn `UserConstructionScript`
  (bind _returnvalue (`PrimitiveComponent.CreateDynamicMaterialInstance` (`self.MeshComponent`) 0 "/Game/Materials/M_Base_Inst.M_Base_Inst" "None"))
  (set `self.DynamicMaterial` _returnvalue))