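; Game mode for a two-player match on a shared camera, handling startup, player deaths and match end.
; BeginPlay shows a fade and the main HUD, passes the first CameraActor to player controllers, and spawns three AI character types inside that per-player loop.
; On death it shows that player's death message and restores their HP.
; Game end swaps the HUD for a score screen, shows the cursor, then disables pawn collision and unpossesses pawns.
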(event `self.AdditionalEvent_OnGameEnded`
  (bind _returnvalue (`|CreateWidget` "/Game/Widget/BP_ResultHudWidget.BP_ResultHudWidget_C"))
  (`/Game/Widget/BP_ResultHudWidget.SetScore` _returnvalue (`self.StatusP1`) (`self.StatusP2`))
  (`UserWidget.AddToViewport` _returnvalue 0)
  (set `PlayerController.bShowMouseCursor` true (`GameplayStatics.GetPlayerController` 0))
  (bind _outactors (`GameplayStatics.GetAllActorsOfClass` "/Game/Blueprints/BP_LMPawnPlayer.BP_LMPawnPlayer_C"))
  (for _array_element _outactors
    (`self.SetActorEnableCollision` _array_element false)
    (bind _returnvalue_2 (`Pawn.GetController` _array_element))
    (if (`KismetSystemLibrary.IsValid` _returnvalue_2)
      (`Controller.UnPossess` _returnvalue_2)))
  (`Widget.RemoveFromParent` (`self.GetMainHUD`)))

(event `self.Event_OnPlayerDied`
  (params (inputIndex :type Integer))
  (`parent.Event_OnPlayerDied` inputIndex)
  (switch `int` inputIndex
    (:`0`
      (bind _returnvalue (`|CreateWidget` "/Game/Widget/BP_PostMessageWidget_1p.BP_PostMessageWidget_1p_C"))
      (`/Game/Widget/BP_PostMessageWidget_1p.Initalize` _returnvalue 2.0 "죽음")
      (`UserWidget.AddToViewport` _returnvalue 0))
    (:`1`
      (bind _returnvalue_2 (`|CreateWidget` "/Game/Widget/BP_PostMessageWidget_2p.BP_PostMessageWidget_2p_C"))
      (`/Game/Widget/BP_PostMessageWidget_2p.Initalize` _returnvalue_2 2.0 "죽음")
      (`UserWidget.AddToViewport` _returnvalue_2 0)))
  (bind _outactors (`GameplayStatics.GetAllActorsOfClass` "/Game/Blueprints/BP_LMPawnPlayer.BP_LMPawnPlayer_C"))
  (for _array_element _outactors
    (if (== (`LMPawnPlayer.PlayerIndex` _array_element) inputIndex)
      (`/Game/Blueprints/BP_LMPawnPlayer.SetFullHP` _array_element inputIndex)
      (break))))

(event `self.ReceiveBeginPlay`
  (`parent.ReceiveBeginPlay`)
  (bind _returnvalue (`|CreateWidget` "/Game/Widget/BP_FadeWidget.BP_FadeWidget_C"))
  (`UserWidget.AddToViewport` _returnvalue 0)
  (`KismetSystemLibrary.Delay` 0.3)
  (`self.ShowOrCreateMainHUD` true)
  (bind _outactors (`GameplayStatics.GetAllActorsOfClass` "/Script/Engine.CameraActor"))
  (if (`KismetArrayLibrary.Array_IsValidIndex` _outactors)
    (bind _output_get (set `self.SharedCamera` (`|GetArrayItem` _outactors)))
    (bind _outactors_2 (`GameplayStatics.GetAllActorsOfClass` "/Game/Blueprints/BP_LMPawnPlayer.BP_LMPawnPlayer_C"))
    (for _array_element _outactors_2
      (bind _asbp_lmplayer_controller (cast `/Game/Blueprints/BP_LMPlayerController` (`Pawn.GetController` _array_element)))
      (`/Game/Blueprints/BP_LMPlayerController.CallServerFunction` _asbp_lmplayer_controller _output_get)
      (`|SpawnActorFromClass` "/Game/Blueprints/BP_MyAICharacter.BP_MyAICharacter_C" (`KismetMathLibrary.MakeTransform` (0.0 0.0 0.0)) "Undefined" "MultiplyWithRoot" null null)
      (`|SpawnActorFromClass` "/Game/Blueprints/BP_MyAICharacter1.BP_MyAICharacter1_C" (`KismetMathLibrary.MakeTransform` (0.0 0.0 0.0)) "Undefined" "MultiplyWithRoot" null null)
      (`|SpawnActorFromClass` "/Game/Blueprints/BP_MyAICharacter2.BP_MyAICharacter2_C" (`KismetMathLibrary.MakeTransform` (0.0 0.0 0.0)) "Undefined" "MultiplyWithRoot" null null))))

(fn `UserConstructionScript`)