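; Player pawn Blueprint that handles the fire input.
; The IA_Fire Started event calls Fire, which is not defined in this graph.
; The Horizontal and Vertical axis events are empty.
; Disconnected nodes for up/right movement input and for spawning BP_Bullet at FIrePosition remain in the graph but never run.
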(event `InputAxis|Horizontal`
  (params (AxisValue :type "Float (single-precision)")))

(event `InputAxis|Vertical`
  (params (AxisValue :type "Float (single-precision)")))

(event `EnhancedInput|/Game/Inputs/IA_Fire`
  (params (ActionValue :type Boolean) (ElapsedSeconds :type "Float (double-precision)") (TriggeredSeconds :type "Float (double-precision)") (InputAction :type "InputAction Object Reference" :default "/Game/Inputs/IA_Fire.IA_Fire"))
  (:`Started`
    (`self.Fire`)))

(fn `UserConstructionScript`)