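; Game mode Blueprint for a two-player match that sets up the shared camera, spawns AI and shows death and result UI.
; BeginPlay takes the first CameraActor, passes it to the first player controller's server function, then spawns three AI characters.
; Player death calls the parent handler and shows a timed "죽음" (death) message in that player's widget.
; Game end displays both players' scores and enables the mouse cursor.
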(event `self.Event_OnPlayerDied`
  (params (inputIndex :type Integer))
  (`parent.Event_OnPlayerDied` inputIndex)
  (switch `int` inputIndex
    (:`0`
      (bind _returnvalue (`|CreateWidget` "/Game/Widget/BP_PostMessageWidget_1p.BP_PostMessageWidget_1p_C"))
      (`/Game/Widget/BP_PostMessageWidget_1p.Initalize` _returnvalue 2.0 "죽음")
      (`UserWidget.AddToViewport` _returnvalue 0))
    (:`1`
      (bind _returnvalue_2 (`|CreateWidget` "/Game/Widget/BP_PostMessageWidget_2p.BP_PostMessageWidget_2p_C"))
      (`/Game/Widget/BP_PostMessageWidget_2p.Initalize` _returnvalue_2 2.0 "죽음")
      (`UserWidget.AddToViewport` _returnvalue_2 0))))

(event `self.AdditionalEvent_OnGameEnded`
  (bind _returnvalue (`|CreateWidget` "/Game/Widget/BP_ResultHudWidget.BP_ResultHudWidget_C"))
  (`/Game/Widget/BP_ResultHudWidget.SetScore` _returnvalue (`self.StatusP1`) (`self.StatusP2`))
  (`UserWidget.AddToViewport` _returnvalue 0)
  (set `PlayerController.bShowMouseCursor` true (`GameplayStatics.GetPlayerController` 0)))

(event `self.ReceiveBeginPlay`
  (bind _outactors (`GameplayStatics.GetAllActorsOfClass` "/Script/Engine.CameraActor"))
  (if (`KismetArrayLibrary.Array_IsValidIndex` _outactors)
    (set `self.SharedCamera` (`|GetArrayItem` _outactors))
    (bind _asbp_lmplayer_controller (cast `/Game/Blueprints/BP_LMPlayerController` (`GameplayStatics.GetPlayerController` 0)))
    (`/Game/Blueprints/BP_LMPlayerController.CallServerFunction` _asbp_lmplayer_controller (`self.SharedCamera`))
    (`|SpawnActorFromClass` "/Game/Blueprints/BP_MyAICharacter.BP_MyAICharacter_C" (`KismetMathLibrary.MakeTransform` (0.0 0.0 0.0)) "Undefined" "MultiplyWithRoot" null null)
    (`|SpawnActorFromClass` "/Game/Blueprints/BP_MyAICharacter1.BP_MyAICharacter1_C" (`KismetMathLibrary.MakeTransform` (0.0 0.0 0.0)) "Undefined" "MultiplyWithRoot" null null)
    (`|SpawnActorFromClass` "/Game/Blueprints/BP_MyAICharacter2.BP_MyAICharacter2_C" (`KismetMathLibrary.MakeTransform` (0.0 0.0 0.0)) "Undefined" "MultiplyWithRoot" null null)))

(fn `UserConstructionScript`)