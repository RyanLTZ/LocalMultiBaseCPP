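; BP_SoundPlayerActor is an actor that plays background music through an Audio component, with controls to set the track, play it and set volume.
; FadeInBGM and FadeOutBGM snap the volume to silent or full, then set mutually exclusive flags.
; Tick steps the volume multiplier by delta time times FadeSpeed until it reaches the limit and clears the flag.
; Fading out only lowers volume and never stops playback.
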(event `FadeOutPlay`
  (params (Delta :type "Float (double-precision)"))
  (bind _audio (`self.Audio`))
  (bind _volumemultiplier (`AudioComponent.VolumeMultiplier` _audio))
  (if (<= _volumemultiplier 0.0)
    (`AudioComponent.SetVolumeMultiplier` _audio 0.0)
    (set `self.IsFadeOut` false)
    (else
      (`AudioComponent.SetVolumeMultiplier` _audio (- _volumemultiplier (* Delta (`self.FadeSpeed`)))))))

(event `self.ReceiveTick`
  (params (DeltaSeconds :type "Float (single-precision)"))
  (if (`self.IsFadeOut`)
    (`self.FadeOutPlay` DeltaSeconds)
    (elif (`self.IsFadeIn`)
      (`self.FadeInPlay` DeltaSeconds))))

(event `FadeInPlay`
  (params (Delta :type "Float (double-precision)"))
  (bind _audio (`self.Audio`))
  (bind _volumemultiplier (`AudioComponent.VolumeMultiplier` _audio))
  (if (>= _volumemultiplier 1.0)
    (`AudioComponent.SetVolumeMultiplier` _audio 1.0)
    (set `self.IsFadeIn` false)
    (else
      (`AudioComponent.SetVolumeMultiplier` _audio (+ _volumemultiplier (* Delta (`self.FadeSpeed`)))))))

(event `SetVolume`
  (params (InputVolume :type "Float (double-precision)"))
  (`AudioComponent.SetVolumeMultiplier` (`self.Audio`) InputVolume))

(event `PlayBGM`
  (`AudioComponent.Play` (`self.Audio`) 0.0))

(event `SetBGM`
  (params (InputSound :type "SoundBase Object Reference"))
  (`AudioComponent.SetSound` (`self.Audio`) InputSound))

(event `FadeOutBGM`
  (set `self.IsFadeOut` true)
  (`AudioComponent.SetVolumeMultiplier` (`self.Audio`) 1.0)
  (set `self.IsFadeIn` false))

(event `FadeInBGM`
  (set `self.IsFadeIn` true)
  (`AudioComponent.SetVolumeMultiplier` (`self.Audio`) 0.0)
  (set `self.IsFadeOut` false))

(fn `UserConstructionScript`)